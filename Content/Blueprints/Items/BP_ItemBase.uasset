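; BP_ItemBase is a base item Blueprint with a Paper2D flipbook and a box trigger for interaction.
; On BeginPlay, it applies a looping setting to the flipbook, then either plays it from the start or holds it stopped on the first frame, depending on an auto-start setting.
; When a PaperCharacter begins overlapping the box, it calls Interact, which is described as an interface method shared by all items.
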(event OnComponentBeginOverlap(BoxCollider)
  (params (OverlappedComponent :type Primitive%20Component%20Object%20Reference) (OtherActor :type Actor%20Object%20Reference) (OtherComp :type Primitive%20Component%20Object%20Reference) (OtherBodyIndex :type Integer) (bFromSweep :type Boolean) (SweepResult :type Hit%20Result%20Structure%20%28by%20ref%29))
  ;[0 0 0] la methode d'interface : interact commune à tous les ItemBase
  (Utilities|Casting|CastToPaperCharacter OtherActor)
  (CallFunction|Interact))

(event EventBeginPlay
  ;[0 0 0] Donne la possibilité de paramétrer un objet à savoir newLooping "si l'anim se joue en boucle" et newAutoStart "si l'anim joue son animd'entréede jeu"
  (Components|Timeline|SetLooping (Variables|Default|GetPaperFlipbook) (Variables|Init|GetNew%20Looping))
  (if (Variables|Init|GetNew%20AutoStart)
    (Components|Timeline|PlayfromStart (Variables|Default|GetPaperFlipbook))
    (else
      (Class|PaperFlipbookComponent|SetPlaybackPositioninFrames (Variables|Default|GetPaperFlipbook) 0 false)
      (Audio|Components|Audio|Stop (Variables|Default|GetPaperFlipbook)))))

(fn ConstructionScript)