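; BP_HealthCollectible is a Paper2D melon pickup that heals the player when interacted with.
; Interact heals through the player's health component, registers the melon on the player and plays a power-up sound.
; It then disables box collision, plays a one-shot collected flipbook and destroys the actor after a short delay.
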(event EventBeginPlay
  (|CallParentFunction))

(event EventInteract
  ;[0 0 0] heal
  (Default|Heal (Variables|/Game/Blueprints/BP_PaperCharacterBase.BP_PaperCharacterBase_C|GetBPC_HealthComponent (CallFunction|GetPaperPlayer)) (Variables|Init|GetHealValue))
  ;[0 0 0] Melon
  (Default|CollectMelon (CallFunction|GetPaperPlayer))
  ;[0 0 0] Play sfx
  (CallFunction|PlaySfx "/Game/Assets/Sounds/powerUp.powerUp" 0.0)
  ;[0 0 0] Anim
  (Collision|SetCollisionEnabled (Variables|Default|GetBoxCollider) "NoCollision")
  (Components|Timeline|SetLooping (Variables|Default|GetPaperFlipbook) false)
  (Sprite|SetFlipbook (Variables|Default|GetPaperFlipbook) (Variables|Default|GetCollectedAnimation))
  (Components|Timeline|PlayfromStart (Variables|Default|GetPaperFlipbook))
  (Utilities|FlowControl|Delay 0.5)
  ;[0 0 0] destroy
  (Actor|DestroyActor))

(fn ConstructionScript
  (|CallParentFunction))