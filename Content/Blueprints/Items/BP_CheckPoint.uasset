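; BP_CheckPoint is a checkpoint item with a flag flipbook that can register itself as the last checkpoint.
; The player's first overlap with the box collider plays the flag-out animation, guarded by IsActivated to run only once.
; When that animation finishes, a bound event swaps the flipbook to a looping idle.
; A separate Interact event passes the actor's first tag to UpdateLastCheckPoint and prints a debug message.
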(event OnComponentBeginOverlap(BoxCollider)
  (params (OverlappedComponent :type Primitive%20Component%20Object%20Reference) (OtherActor :type Actor%20Object%20Reference) (OtherComp :type Primitive%20Component%20Object%20Reference) (OtherBodyIndex :type Integer) (bFromSweep :type Boolean) (SweepResult :type Hit%20Result%20Structure%20%28by%20ref%29))
  ;[0 0 0] On active qu'une seule fois le start de l'anim de "idle" qui ensuite joue en boucle
  (if (and (== OtherActor (CallFunction|GetPaperPlayer)) (not (Variables|Default|GetisActivated)))
    (Components|Timeline|PlayfromStart (Variables|Default|GetPaperFlipbook))
    (Variables|Default|SetisActivated true)))

(event Custom|onAnimationFinished
  ;[0 0 0] lorsque le drapeau est sorti, on change le flipbook pour celui du idle
  (Sprite|SetFlipbook (Variables|Default|GetPaperFlipbook) "/Game/Assets/Flipbooks/Checkpoint-idle.Checkpoint-idle")
  (Components|Timeline|SetLooping (Variables|Default|GetPaperFlipbook) true)
  (Components|Timeline|PlayfromStart (Variables|Default|GetPaperFlipbook)))

(event EventBeginPlay
  (|CallParentFunction)
  ;[0 0 0] lorsque le drapeau est sorti, on change le flipbook pour celui du idle
  (EventDispatchers|BindEventtoOnFinishedPlaying (Variables|Default|GetPaperFlipbook) (delegate Custom|onAnimationFinished)))

(event EventInteract
  (CallFunction|UpdateLastCheckPoint (Utilities|Array|Get(acopy) (Variables|Default|GetTags)))
  (Development|PrintString (Utilities|String|Append "nouveau check point" " : " (Utilities|String|ToString(Name) (Utilities|Array|Get(acopy) (Variables|Default|GetTags)))) true true "(R=0.802083,G=0.476757,B=0.115698,A=1.000000)"))

(fn ConstructionScript
  (|CallParentFunction))