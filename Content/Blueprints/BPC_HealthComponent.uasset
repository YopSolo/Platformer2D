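; Health component that tracks damage taken and death state for its owning actor.
; Current HP and HP ratio derive from max HP minus accumulated damage, which DoDamage clamps before setting the dead flag.
; Heal sends negative damage to the owner through ApplyDamage rather than calling DoDamage, and no damage event is bound in this component.
; The dead flag can also be set directly.
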(event EventBeginPlay)

(event EventTick
  (params (DeltaSeconds :type Float%20%28single-precision%29)))

(fn GetHp
  (return (- (Variables|Default|GetMaxHP) (Variables|Default|GetCurrentDamage))))

(fn GetHpRatio
  (return (/ (CallFunction|GetHp) (Variables|Default|GetMaxHP))))

(fn Heal
  (params (Amount :type Float%20%28single-precision%29))
  (Game|Damage|ApplyDamage (Components|GetOwner) (* Amount -1.0) 0 0))

(fn GetIsDead
  (return (Variables|Default|GetisDead?)))

(fn SetIsDead
  (params (isDead? :type Boolean))
  (Variables|Default|SetisDead? isDead?))

(fn DoDamage
  (params (amount :type Float%20%28single-precision%29))
  (bind _output_get (Variables|Default|SetcurrentDamage (Math|Float|Clamp(Float) (+ amount (Variables|Default|GetcurrentDamage)) 0.0 (Variables|Default|GetMaxHp))))
  (Variables|Default|SetisDead? (>= _output_get (Variables|Default|GetMaxHp))))