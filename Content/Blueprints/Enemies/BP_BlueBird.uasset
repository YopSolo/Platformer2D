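; Blue bird enemy for a 2D Paper2D game that moves horizontally and reverses direction when it hits an obstacle.
; Tick feeds constant movement input along X, and capsule hits on anything but the player with a sideways normal toggle the direction.
; A DoOnce reset after a short delay debounces turns, and the sprite mirrors through its X scale.
; Parent enemy animation functions are overridden to use the bird's flying and hit flipbooks.
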(event OnComponentHit(CapsuleComponent)
  (params (HitComponent :type Primitive%20Component%20Object%20Reference) (OtherActor :type Actor%20Object%20Reference) (OtherComp :type Primitive%20Component%20Object%20Reference) (NormalImpulse :type Vector :default "0, 0, 0") (Hit :type Hit%20Result%20Structure%20%28by%20ref%29))
  ;[0 0 0] Collision
  (if (!= OtherActor (Game|Player|GetPlayerPawn 0))
    (if (!= (.X (Math|Vector|BreakVector (.normal Hit))) 0.0)
      (Utilities|FlowControl|DoOnce false
        (:Completed
          (Variables|Default|SetisMovingRight (not (Variables|Default|GetisMovingRight)))
          (CallFunction|UpdateFacingRotation)
          (Utilities|FlowControl|Delay 0.2)
          (CallFunction|ResetCollisionCheck))))))

(event Custom|ResetCollisionCheck
  (Utilities|FlowControl|DoOnce false) ; enters at Reset
)

(event EventTick
  (params (DeltaSeconds :type Float%20%28single-precision%29))
  ;[0 0 0] Déplacement
  (Pawn|Input|AddMovementInput "1.000000, 0, 0" (select (Variables|Default|GetisMovingRight) 1.0 -1.0) false))

(event EventBeginPlay
  ;[0 0 0] Oriente le Sprite dans la bonne direction
  (CallFunction|UpdateFacingRotation))

(fn ConstructionScript
  (|CallParentFunction)
  (Sprite|SetFlipbook (Variables|Default|GetSprite) (Variables|Default|GetbaseAnimation)))

(fn UpdateFacingRotation
  (bind _sprite (Variables|Default|GetSprite))
  (bind _returnvalue (Transformation|GetWorldScale _sprite))
  (Transformation|SetWorldScale3D (Variables|Default|GetSprite) (Math|Vector|MakeVector (* (Math|Float|Absolute(Float) (.x _returnvalue)) (select (Variables|Default|GetisMovingRight) -1.0 1.0)) (.y _returnvalue) (.z _returnvalue))))

(fn PlayEnemyDamagedAnimation
  (params (NewFlipbook :type Paper%20Flipbook%20Object%20Reference))
  (|CallParentFunction "/Game/Assets/Flipbooks/FB-BB-hit.FB-BB-hit"))

(fn PlayBaseAnimation
  (params (NewFlipbook :type Paper%20Flipbook%20Object%20Reference))
  (|CallParentFunction "/Game/Assets/Flipbooks/FB-bb-Flying.FB-BB-Flying"))