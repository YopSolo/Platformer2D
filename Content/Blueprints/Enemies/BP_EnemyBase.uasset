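; BP_EnemyBase is a Paper2D enemy base that reacts to damage through flipbook animations and sound effects.
; AnyDamage passes damage to BPCHealthComponent unless already dead, then checks for death.
; Surviving hits play a hurt flipbook and sound, then restore the looping base animation after a short delay.
; Death disables capsule and box collision, plays the death flipbook with an explosion sound, and destroys the actor after a delay.
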(event Game|Damage|EventAnyDamage
  (params (Damage :type Float%20%28single-precision%29) (DamageType :type Damage%20Type%20Object%20Reference) (InstigatedBy :type Controller%20Object%20Reference) (DamageCauser :type Actor%20Object%20Reference))
  (if (not (Default|GetIsDead (Variables|Default|GetBPC_HealthComponent)))
    (Default|DoDamage (Variables|Default|GetBPC_HealthComponent) Damage)
    (if (Default|GetIsDead (Variables|Default|GetBPC_HealthComponent))
      (CallFunction|PlayEnemyDiedAnimation (Variables|Default|GetdeathAnimation))
      ;[1 0.1269 0.916] Sfx
      (CallFunction|PlaySfx "/Game/Assets/Sounds/explosion.explosion" 0.0)
      (Utilities|FlowControl|Delay 0.5)
      (Actor|DestroyActor)
      (else
        (CallFunction|PlayEnemyDamagedAnimation (Variables|Default|GetdamagedAnimation))
        (CallFunction|PlaySfx "/Game/Assets/Sounds/hitHurt.hitHurt" 0.0)
        (Utilities|FlowControl|Delay 0.5)
        (CallFunction|PlayBaseAnimation (Variables|Default|GetbaseAnimation))))))

(fn ConstructionScript)

(fn PlayEnemyDiedAnimation
  (params (NewFlipbook :type Paper%20Flipbook%20Object%20Reference))
  (Collision|SetCollisionEnabled (Variables|Collision|GetCapsuleComponent) "NoCollision")
  (Collision|SetCollisionEnabled (Variables|Default|GetCollisionBox) "NoCollision")
  (Components|Timeline|SetLooping (Variables|Default|GetSprite) false)
  (Sprite|SetFlipbook (Variables|Default|GetSprite) NewFlipbook)
  (Components|Timeline|PlayfromStart (Variables|Default|GetSprite)))

(fn PlayEnemyDamagedAnimation
  (params (NewFlipbook :type Paper%20Flipbook%20Object%20Reference))
  (Components|Timeline|SetLooping (Variables|Default|GetSprite) false)
  (Sprite|SetFlipbook (Variables|Default|GetSprite) NewFlipbook)
  (Components|Timeline|PlayfromStart (Variables|Default|GetSprite)))

(fn PlayBaseAnimation
  (params (NewFlipbook :type Paper%20Flipbook%20Object%20Reference))
  (Components|Timeline|SetLooping (Variables|Default|GetSprite) true)
  (Sprite|SetFlipbook (Variables|Default|GetSprite) NewFlipbook)
  (Components|Timeline|PlayfromStart (Variables|Default|GetSprite)))